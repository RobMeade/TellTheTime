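; Game mode for a level-based quiz game, running question flow, star scoring, level unlocking, saving and music.
; It binds to BP_PlayerController events, deferring game setup until UI widgets initialise, and broadcasts state changes through its own dispatchers.
; Levels load from DT_Levels, and unlocks are rebuilt from star achievements saved in SG_SaveGame.
; Completing a level awards 0–3 stars by correct-answer ratio, unlocking the next when the threshold is met.
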(event EventBeginPlay
  ;[1 1 1] Initialise
  (CallFunction|SetReferences)
  (CallFunction|BindtoEvents))

(fn ConstructionScript)

(fn AwardStars
  ;[1 1 1] Award Stars
  (bind _percent (CallFunction|GetLevelCorrectAnswersasPercent))
  (bind _achievedstars (CallFunction|CalculateAchievedStars _percent))
  (Default|CallStarsAwarded (.ID (Utilities|Struct|BreakSLevel (Variables|Game|GetCurrentLevel))) _achievedstars)
  (return _achievedstars))

(fn BindtoEvents
  ;[1 1 1] Bind to Events
  (EventDispatchers|BindEventtoPlayerControllerInitialised (Variables|References|GetPlayerController) (EventDispatchers|CreateEvent :!event OnPlayerControllerInitialised))
  (EventDispatchers|BindEventtoUIWidgetsInitialised (Variables|References|GetPlayerController) (EventDispatchers|CreateEvent :!event OnUIWidgetsInitialised))
  (EventDispatchers|BindEventtoLevelSelectionChanged (Variables|References|GetPlayerController) (EventDispatchers|CreateEvent :!event OnLevelSelectionChanged))
  (EventDispatchers|BindEventtoLearningObjectiveContinueClicked (Variables|References|GetPlayerController) (EventDispatchers|CreateEvent :!event OnLearningObjectiveContinueClicked))
  (EventDispatchers|BindEventtoAnswerSelected (Variables|References|GetPlayerController) (EventDispatchers|CreateEvent :!event OnAnswerSelected))
  (EventDispatchers|BindEventtoResultContinueClicked (Variables|References|GetPlayerController) (EventDispatchers|CreateEvent :!event OnResultContinueClicked))
  (EventDispatchers|BindEventtoMusicVolumeChanged (Variables|References|GetPlayerController) (EventDispatchers|CreateEvent :!event OnMusicVolumeChanged))
  (EventDispatchers|BindEventtoPlayerPreferencesChanged (Variables|References|GetPlayerController) (EventDispatchers|CreateEvent :!event OnPlayerPreferencesChanged))
  (EventDispatchers|BindEventtoResetPlayerProgressSelected (Variables|References|GetPlayerController) (EventDispatchers|CreateEvent :!event OnResetPlayerProgress))
  (EventDispatchers|BindEventtoLevelAchievementChanged (Variables|References|GetPlayerController) (EventDispatchers|CreateEvent :!event OnLevelAchievementChanged)))

(fn CalculateAchievedStars
  (params (CorrectAnswersAsPercent :type Float%20%28single-precision%29))
  ;[1 1 1] Calculate Achieved Stars
  (if (== CorrectAnswersAsPercent 0.0)
    (return 0)
    (elif (and (> CorrectAnswersAsPercent 0.0) (< CorrectAnswersAsPercent 0.5))
      (return 1)
      (elif (and (>= CorrectAnswersAsPercent 0.5) (< CorrectAnswersAsPercent 1.0))
        (return 2)
        (elif (== CorrectAnswersAsPercent 1.0)
          (return 3))))))

(fn OnAnswerSelected
  (params (IsAnswerCorrect :type Boolean))
  ;[1 1 1] Answer Selected
  (if IsAnswerCorrect
    (Math|Integer|IncrementInt (Variables|Game|GetCorrectAnswersThisLevel)
      (:%20%20
        _)))
  (Default|CallResultChanged IsAnswerCorrect))

(fn OnLearningObjectiveContinueClicked
  ;[1 1 1] Learning Objective Continue Clicked
  (bind _question (CallFunction|GetQuestionbyIndex))
  (Default|CallQuestionChanged _question))

(fn GameHasMoreLevels
  ;[1 1 1] Game Has More Levels?
  (return (< (Variables|Game|GetCurrentLevelIndex) (Utilities|Array|LastIndex (Variables|Game|GetLevels)))))

(fn GetDefaultPlayerData
  ;[1 1 1] Get Default Player Data
  (return (Utilities|Struct|MakeSPlayerData) (Utilities|Struct|MakeSPlayerPreferences (Variables|Config|Audio|GetDefaultMusicVolume) false (Variables|Config|Audio|GetDefaultSFXVolume) false (Variables|Config|Audio|GetDefaultNarrationVolume))))

(fn GetLevelbyIndex
  (params (Index :type Integer))
  ;[1 1 1] Get Level by Index
  (return (Utilities|Array|Get(acopy) (Variables|Game|GetLevels) Index)))

(fn GetLevelCorrectAnswersasPercent
  ;[1 1 1] Get Correct Answers as a Percent for the Current Level
  (return (/ (Math|Conversions|ToFloat(Integer) (Variables|Game|GetCorrectAnswersThisLevel)) (Math|Conversions|ToFloat(Integer) (Utilities|Array|Length (.Questions (Utilities|Struct|BreakSLevel (Variables|Game|GetCurrentLevel))))))))

(fn GetQuestionbyIndex
  ;[1 1 1] Get Question
  (return (Utilities|Array|Get(acopy) (.Questions (Utilities|Struct|BreakSLevel (Variables|Game|GetCurrentLevel))) (Variables|Game|GetCurrentQuestionIndex))))

(fn GetRandomLevelFeedbackbyStarsAchieved
  (params (StarsAchieved :type Integer))
  (bind _levelfeedback0stars (Variables|Config|Game|GetLevelFeedback0Stars))
  (bind _levelfeedback1star (Variables|Config|Game|GetLevelFeedback1Star))
  (bind _levelfeedback2stars (Variables|Config|Game|GetLevelFeedback2Stars))
  (bind _levelfeedback3stars (Variables|Config|Game|GetLevelFeedback3Stars))
  (bind _returnvalue (Utilities|Select :Index StarsAchieved :Option%200 _levelfeedback0stars :Option%201 _levelfeedback1star :Option%202 _levelfeedback2stars :Option%203 _levelfeedback3stars))
  ;[1 1 1] Get Random Level Feedback by Stars Achieved
  (return (Utilities|Array|Get(acopy) _returnvalue (Math|Random|RandomIntegerinRange 0 (- (Utilities|Array|Length _returnvalue) 1)))))

(fn GetSafeVolumeMultiplier
  (params (Volume :type Float%20%28single-precision%29))
  ;[1 1 1] Get Safe Volume Multiplier
  (if (== Volume 0.0)
    (return 0.001)
    (else
      (return Volume))))

(fn GetStars
  ;[1 1 1] Get Stars
  (bind _currentstars (Default|GetCurrentStars (Variables|References|GetPlayerController)))
  (return _currentstars (* (Utilities|Array|Length (Variables|Game|GetLevels)) 3)))

(fn InitialiseGame
  ;[1 1 1] Initialise Game
  (CallFunction|InitialiseSaveGame)
  (CallFunction|LoadLevelData)
  (CallFunction|UnlockLevel)
  (CallFunction|LoadPlayerData)
  (CallFunction|UpdatePlayerProgression)
  (CallFunction|PlayMusic))

(fn InitialiseSaveGame
  ;[1 1 1] Initialise Save Game
  (bind (_playerdata _playerpreferences) (CallFunction|GetDefaultPlayerData))
  (Default|Initialise (Variables|SaveGame|GetSaveGame) _playerdata _playerpreferences))

(fn InitialiseUI
  ;[1 1 1] Initialise UI
  (Default|InitialiseUI (Variables|References|GetPlayerController)))

(fn IsNextLevelUnlocked
  ;[1 1 1] Is Next Level Unlocked
  (bind _level (CallFunction|GetLevelbyIndex (+ (Variables|Game|GetCurrentLevelIndex) 1)))
  (return (.IsUnlocked (Utilities|Struct|BreakSLevel _level))))

(fn LevelComplete
  (bind _currentlevel (Variables|Game|GetCurrentLevel))
  ;[1 1 1] Level Complete
  (bind _stars (CallFunction|AwardStars))
  (bind _output_get (LocalVariables|SetStarsAchieved _stars))
  (if (>= _output_get (Variables|Config|Game|GetStarsToUnlockLevel))
    (bind _morelevels (CallFunction|GameHasMoreLevels))
    (if _morelevels
      (bind _levelisunlocked (CallFunction|IsNextLevelUnlocked))
      (if _levelisunlocked
        (LocalVariables|SetLevelOutcomeState "NewEnumerator3")
        (else
          (CallFunction|UnlockNextLevel)
          (LocalVariables|SetLevelOutcomeState "NewEnumerator2")))
      (else
        (LocalVariables|SetLevelOutcomeState "NewEnumerator1")))
    (else
      (LocalVariables|SetLevelOutcomeState "NewEnumerator0")))
  (Default|CallLevelCompleted (Utilities|Struct|MakeSLevelCompleteSummary (.id _currentlevel) (LocalVariables|GetStarsAchieved) (Variables|Game|GetCorrectAnswersThisLevel) (Utilities|Array|Length (.questions _currentlevel)) (LocalVariables|GetLevelOutcomeState))))

(fn LevelHasMoreQuestions
  ;[1 1 1] Level Has More Questions?
  (return (< (Variables|Game|GetCurrentQuestionIndex) (Utilities|Array|LastIndex (.Questions (Utilities|Struct|BreakSLevel (Variables|Game|GetCurrentLevel)))))))

(fn OnLevelAchievementChanged
  (params (LevelID :type Integer))
  ;[1 1 1] Save Player Data
  (CallFunction|SavePlayerData))

(fn OnLevelSelectionChanged
  (params (LevelIndex :type Integer))
  ;[1 1 1] Level Selection Changed
  (bind _output_get (Variables|Game|SetCurrentLevelIndex LevelIndex))
  (bind _level (CallFunction|GetLevelbyIndex _output_get))
  (bind _output_get_2 (Variables|Game|SetCurrentLevel _level))
  (Variables|Game|SetCurrentQuestionIndex 0)
  (Variables|Game|SetCorrectAnswersThisLevel 0)
  (Default|CallLevelChanged _output_get_2))

(fn OnMusicVolumeChanged
  (params (Volume :type Float%20%28single-precision%29) (IsMuted :type Boolean))
  ;[1 1 1] Music Volume Changed
  (bind _safevolumemultiplier (CallFunction|GetSafeVolumeMultiplier (select IsMuted 0.0 Volume)))
  (Audio|Components|Audio|SetVolumeMultiplier (Variables|Default|GetMusic) _safevolumemultiplier :!class /Script/Engine.AudioComponent))

(fn OnPlayerControllerInitialised
  ;[1 1 1] Initialise UI
  (CallFunction|InitialiseUI))

(fn OnPlayerPreferencesChanged
  ;[1 1 1] Save Player Data
  (CallFunction|SavePlayerData))

(fn OnResetPlayerProgress
  (bind _playercontroller (Variables|References|GetPlayerController))
  ;[1 1 1] Reset Player Progress
  (CallFunction|LoadLevelData)
  (CallFunction|UnlockLevel)
  (bind _playerdata (CallFunction|GetDefaultPlayerData))
  (bind _output_get (Variables|/Game/Blueprints/BP_PlayerController.BP_PlayerController_C|SetPlayerData _playercontroller _playerdata))
  (Default|SaveData (Variables|SaveGame|GetSaveGame) _output_get (Variables|/Game/Blueprints/BP_PlayerController.BP_PlayerController_C|GetPlayerPreferences _playercontroller))
  (CallFunction|UpdatePlayerProgression))

(fn OnResultContinueClicked
  ;[1 1 1] Result Continue Button Clicked
  (bind _morequestions (CallFunction|LevelHasMoreQuestions))
  (if _morequestions
    (CallFunction|NextQuestion)
    (else
      (CallFunction|LevelComplete))))

(fn OnUIWidgetsInitialised
  ;[1 1 1] Initialise Game
  (CallFunction|InitialiseGame))

(fn LoadLevelData
  ;[1 1 1] Load Level Data
  (Utilities|Array|Clear (Variables|Game|GetLevels))
  (bind _outrownames (DataTable|GetDataTableRowNames "/Game/DataTables/DT_Levels.DT_Levels"))
  (for _array_element _outrownames
    (bind _returnvalue (Utilities|GetDataTableRow "/Game/DataTables/DT_Levels.DT_Levels" _array_element)
      (:then
        (Utilities|Array|Add (Variables|Game|GetLevels) _returnvalue))))
  (Default|CallLevelDataLoaded))

(fn LoadPlayerData
  ;[1 1 1] Load Player Data
  (bind (_playerdata _playerpreferences) (Default|LoadData (Variables|SaveGame|GetSaveGame)))
  (Default|CallPlayerDataLoaded _playerdata _playerpreferences))

(fn NextQuestion
  ;[1 1 1] Next Question
  (Math|Integer|IncrementInt (Variables|Game|GetCurrentQuestionIndex)
    (:%20%20
      (bind _question (CallFunction|GetQuestionbyIndex))
      (Default|CallQuestionChanged _question)
      (Default|CallNextQuestionSelected))))

(fn PlayMusic
  (bind _playercontroller (Variables|References|GetPlayerController))
  (bind _playerpreferences (Variables|/Game/Blueprints/BP_PlayerController.BP_PlayerController_C|GetPlayerPreferences _playercontroller))
  ;[1 1 1] Play Music
  (bind _safevolumemultiplier (CallFunction|GetSafeVolumeMultiplier (select (.musicismuted _playerpreferences) 0.0 (.musicvolume _playerpreferences))))
  (Audio|Components|Audio|SetVolumeMultiplier (Variables|Default|GetMusic) _safevolumemultiplier :!class /Script/Engine.AudioComponent)
  (Audio|Components|Audio|SetSound (Variables|Default|GetMusic) (Variables|Config|Audio|GetMusicCue))
  (Audio|Components|Audio|Play (Variables|Default|GetMusic) 0.0))

(fn SavePlayerData
  (bind _playercontroller (Variables|References|GetPlayerController))
  ;[1 1 1] Save Player Data
  (Default|SaveData (Variables|SaveGame|GetSaveGame) (Variables|/Game/Blueprints/BP_PlayerController.BP_PlayerController_C|GetPlayerData _playercontroller) (Variables|/Game/Blueprints/BP_PlayerController.BP_PlayerController_C|GetPlayerPreferences _playercontroller)))

(fn SetReferences
  ;[1 1 1] Set References
  (bind _asbp_player_controller (Utilities|Casting|CastToBP_PlayerController (Game|GetPlayerController 0)))
  (Variables|References|SetPlayerController _asbp_player_controller)
  (bind _returnvalue (SaveGame|CreateSaveGameObject "/Game/SaveGame/SG_SaveGame.SG_SaveGame_C"))
  (Variables|SaveGame|SetSaveGame _returnvalue))

(fn UnlockLevel
  (params (LevelIndex :type Integer))
  ;[1 1 1] Unlock Level
  (bind _structout (Utilities|Struct|SetmembersinSLevel (Utilities|Array|Get(acopy) (Variables|Game|GetLevels) LevelIndex) true))
  (Default|CallLevelUnlocked (.id _structout)))

(fn UnlockNextLevel
  ;[1 1 1] Unlock Next Level
  (CallFunction|UnlockLevel (+ (Variables|Game|GetCurrentLevelIndex) 1)))

(fn UpdatePlayerProgression
  ;[1 1 1] Update Player Progression
  (bind (_array_element _array_index) (Utilities|Array|ForEachLoopwithBreak (Variables|Game|GetLevels) :!label _label)
    (:LoopBody
      (LocalVariables|SetArrayElement _array_element)
      (LocalVariables|SetArrayIndex _array_index)
      (Utilities|Struct|SetmembersinSLevel (LocalVariables|GetArrayElement) (LocalVariables|GetCanUnlockNextLevel))
      (bind _hasachievement (Default|HasLevelAchievementforLevelID (Variables|References|GetPlayerController) (.id (LocalVariables|GetArrayElement))))
      (if _hasachievement
        (bind _levelachievement (Default|GetLevelAchievementbyLevelID (Variables|References|GetPlayerController) (.id (LocalVariables|GetArrayElement))))
        (Utilities|Struct|SetmembersinSLevel (LocalVariables|GetArrayElement) (.Stars (Utilities|Struct|BreakSLevelAchievement _levelachievement)))
        (Utilities|Array|SetArrayElem (Variables|Game|GetLevels) (LocalVariables|GetArrayIndex) (LocalVariables|GetArrayElement))
        (LocalVariables|SetCanUnlockNextLevel (>= (.Stars (Utilities|Struct|BreakSLevelAchievement _levelachievement)) 2))
        (else
          (Utilities|Array|SetArrayElem (Variables|Game|GetLevels) (LocalVariables|GetArrayIndex) (LocalVariables|GetArrayElement))
          (goto _label Break))))
    (:Completed
      (Default|CallPlayerProgressionUpdated))))