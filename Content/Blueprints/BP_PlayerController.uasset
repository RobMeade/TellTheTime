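; Player controller for a narrated educational quiz game, driving the menus, level flow and player state.
; InitialiseUI creates all widgets up front, binds their events and switches screens by toggling visibility.
; GameMode events supply player data, advance screens and award stars, keeping each level's best, while its own dispatchers report choices and changes.
; It also plays button and answer SFX plus learning narration, using preferred volumes and voice.
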(event EventBeginPlay
  ;[1 1 1] Initialise
  (CallFunction|SetReferences)
  (CallFunction|BindtoGameModeEvents)
  (Default|CallPlayerControllerInitialised))

(fn ConstructionScript)

(fn AddtoViewportandHide
  (params (UserWidget :type User%20Widget%20Object%20Reference))
  ;[1 1 1] Add to Viewport and Hide
  (UserInterface|Viewport|AddtoViewport UserWidget 0)
  (Widget|SetVisibility UserWidget "Hidden"))

(fn BindtoGameModeEvents
  ;[1 1 1] Bind to GameMode Events
  (EventDispatchers|BindEventtoPlayerDataLoaded (Variables|References|GetGameMode) (EventDispatchers|CreateEvent :!event OnPlayerDataLoaded))
  (EventDispatchers|BindEventtoNextQuestionSelected (Variables|References|GetGameMode) (EventDispatchers|CreateEvent :!event OnNextQuestionSelected))
  (EventDispatchers|BindEventtoLevelCompleted (Variables|References|GetGameMode) (EventDispatchers|CreateEvent :!event OnLevelCompleted))
  (EventDispatchers|BindEventtoStarsAwarded (Variables|References|GetGameMode) (EventDispatchers|CreateEvent :!event OnStarsAwarded))
  (EventDispatchers|BindEventtoLevelChanged (Variables|References|GetGameMode) (EventDispatchers|CreateEvent :!event OnLevelChanged)))

(fn BindtoUIEvents
  ;[1 1 1] Bind to UI Events
  (EventDispatchers|BindEventtoPlayClicked (Variables|References|GetMainMenuWidget) (EventDispatchers|CreateEvent :!event OnMainMenuPlayClicked))
  (EventDispatchers|BindEventtoOptionsClicked (Variables|References|GetMainMenuWidget) (EventDispatchers|CreateEvent :!event OnMainMenuOptionsClicked))
  (EventDispatchers|BindEventtoCreditsClicked (Variables|References|GetMainMenuWidget) (EventDispatchers|CreateEvent :!event OnMainMenuCreditsClicked))
  (EventDispatchers|BindEventtoQuitClicked (Variables|References|GetMainMenuWidget) (EventDispatchers|CreateEvent :!event OnMainMenuQuitClicked))
  (EventDispatchers|BindEventtoMusicVolumeChanged (Variables|References|GetOptionsWidget) (EventDispatchers|CreateEvent :!event OnOptionsMusicVolumeChanged))
  (EventDispatchers|BindEventtoSFXVolumeChanged (Variables|References|GetOptionsWidget) (EventDispatchers|CreateEvent :!event OnOptionsSFXVolumeChanged))
  (EventDispatchers|BindEventtoNarrationVoiceChanged (Variables|References|GetOptionsWidget) (EventDispatchers|CreateEvent :!event OnOptionsNarrationVoiceChanged))
  (EventDispatchers|BindEventtoNarrationVolumeChanged (Variables|References|GetOptionsWidget) (EventDispatchers|CreateEvent :!event OnOptionsNarrationVolumeChanged))
  (EventDispatchers|BindEventtoMainMenuClicked (Variables|References|GetOptionsWidget) (EventDispatchers|CreateEvent :!event OnOptionsMainMenuClicked))
  (EventDispatchers|BindEventtoMainMenuClicked (Variables|References|GetCreditsWidget) (EventDispatchers|CreateEvent :!event OnCreditsMainMenuClicked))
  (EventDispatchers|BindEventtoMainMenuClicked (Variables|References|GetLevelSelectWidget) (EventDispatchers|CreateEvent :!event OnLevelSelectMainMenuClicked))
  (EventDispatchers|BindEventtoLevelSelected (Variables|References|GetLevelSelectWidget) (EventDispatchers|CreateEvent :!event OnLevelButtonClicked))
  (EventDispatchers|BindEventtoLevelSelectClicked (Variables|References|GetLearningObjectiveWidget) (EventDispatchers|CreateEvent :!event OnLearningObjectiveLevelSelectClicked))
  (EventDispatchers|BindEventtoContinueClicked (Variables|References|GetLearningObjectiveWidget) (EventDispatchers|CreateEvent :!event OnLearningObjectiveContinueClicked))
  (EventDispatchers|BindEventtoAnswerSelected (Variables|References|GetQuestionWidget) (EventDispatchers|CreateEvent :!event OnQuestionAnswerClicked))
  (EventDispatchers|BindEventtoLevelSelectClicked (Variables|References|GetQuestionWidget) (EventDispatchers|CreateEvent :!event OnQuestionLevelSelectClicked))
  (EventDispatchers|BindEventtoOnContinueClicked (Variables|References|GetResultWidget) (EventDispatchers|CreateEvent :!event OnResultContinueClicked))
  (EventDispatchers|BindEventtoMainMenuClicked (Variables|References|GetLevelCompleteWidget) (EventDispatchers|CreateEvent :!event OnLevelCompleteMainMenuClicked))
  (EventDispatchers|BindEventtoLevelSelectClicked (Variables|References|GetLevelCompleteWidget) (EventDispatchers|CreateEvent :!event OnLevelCompleteLevelSelectClicked))
  (EventDispatchers|BindEventtoReplayLevelClicked (Variables|References|GetLevelCompleteWidget) (EventDispatchers|CreateEvent :!event OnLevelCompleteReplayLevelClicked))
  (EventDispatchers|BindEventtoContinueClicked (Variables|References|GetLevelCompleteWidget) (EventDispatchers|CreateEvent :!event OnLevelCompleteContinueClicked)))

(fn CreateUIWidgets
  ;[1 1 1] Create UI Widgets
  (bind _returnvalue (UserInterface|CreateWidget "/Game/Widgets/WBP_MainMenu.WBP_MainMenu_C" self))
  (bind _output_get (Variables|References|SetMainMenuWidget _returnvalue))
  (CallFunction|AddtoViewportandHide _output_get)
  (bind _returnvalue_2 (UserInterface|CreateWidget "/Game/Widgets/WBP_Options.WBP_Options_C" self))
  (bind _output_get_2 (Variables|References|SetOptionsWidget _returnvalue_2))
  (CallFunction|AddtoViewportandHide _output_get_2)
  (bind _returnvalue_3 (UserInterface|CreateWidget "/Game/Widgets/WBP_Credits.WBP_Credits_C" self))
  (bind _output_get_3 (Variables|References|SetCreditsWidget _returnvalue_3))
  (CallFunction|AddtoViewportandHide _output_get_3)
  (bind _returnvalue_4 (UserInterface|CreateWidget "/Game/Widgets/WBP_LevelSelect.WBP_LevelSelect_C" self))
  (bind _output_get_4 (Variables|References|SetLevelSelectWidget _returnvalue_4))
  (CallFunction|AddtoViewportandHide _output_get_4)
  (bind _returnvalue_5 (UserInterface|CreateWidget "/Game/Widgets/WBP_LearningObjective.WBP_LearningObjective_C" self))
  (bind _output_get_5 (Variables|References|SetLearningObjectiveWidget _returnvalue_5))
  (CallFunction|AddtoViewportandHide _output_get_5)
  (bind _returnvalue_6 (UserInterface|CreateWidget "/Game/Widgets/WBP_Question.WBP_Question_C" self))
  (bind _output_get_6 (Variables|References|SetQuestionWidget _returnvalue_6))
  (CallFunction|AddtoViewportandHide _output_get_6)
  (bind _returnvalue_7 (UserInterface|CreateWidget "/Game/Widgets/WBP_Result.WBP_Result_C" self))
  (bind _output_get_7 (Variables|References|SetResultWidget _returnvalue_7))
  (CallFunction|AddtoViewportandHide _output_get_7)
  (bind _returnvalue_8 (UserInterface|CreateWidget "/Game/Widgets/WBP_LevelComplete.WBP_LevelComplete_C" self))
  (bind _output_get_8 (Variables|References|SetLevelCompleteWidget _returnvalue_8))
  (CallFunction|AddtoViewportandHide _output_get_8)
  (bind _returnvalue_9 (UserInterface|CreateWidget "/Game/Widgets/WBP_HUD.WBP_HUD_C" self))
  (bind _output_get_9 (Variables|References|SetHUDWidget _returnvalue_9))
  (UserInterface|Viewport|AddtoViewport _output_get_9 0))

(fn GetCurrentStars
  ;[1 1 1] Get Current Stars
  (for _array_element (.levelachievements (Variables|Player|GetPlayerData))
    (LocalVariables|SetStars (+ (LocalVariables|GetStars) (.Stars (Utilities|Struct|BreakSLevelAchievement _array_element)))))
  (return (LocalVariables|GetStars)))

(fn GetLevelAchievementbyLevelID
  (params (LevelID :type Integer))
  ;[1 1 1] Get Level Achievement by Level ID
  (bind _index (CallFunction|GetLevelAchievementIndexbyLevelID LevelID))
  (return (Utilities|Array|Get(acopy) (Utilities|Struct|BreakSPlayerData (Variables|Player|GetPlayerData)) _index)))

(fn GetLevelAchievementIndexbyLevelID
  (params (LevelID :type Integer))
  ;[1 1 1] Get Level Achievement Index by Level ID
  (bind (_array_element _array_index) (Utilities|Array|ForEachLoopwithBreak (Utilities|Struct|BreakSPlayerData (Variables|Player|GetPlayerData)) :!label _label)
    (:LoopBody
      (if (== (.LevelID (Utilities|Struct|BreakSLevelAchievement _array_element)) LevelID)
        (LocalVariables|SetArrayIndex _array_index)
        (goto _label Break)))
    (:Completed
      (return (LocalVariables|GetArrayIndex)))))

(fn HasLevelAchievementforLevelID
  (params (LevelID :type Integer))
  ;[1 1 1] Has Level Achievement for Level ID
  (bind _index (CallFunction|GetLevelAchievementIndexbyLevelID LevelID))
  (return (> _index -1)))

(fn InitialisePlayer
  (params (PlayerData :type S%20Player%20Data%20Structure) (PlayerPreferences :type S%20Player%20Preferences%20Structure))
  ;[1 1 1] Initialise Player
  (Variables|Player|SetPlayerData PlayerData)
  (Variables|Player|SetPlayerPreferences PlayerPreferences))

(fn InitialiseUI
  ;[1 1 1] Initialise UI
  (CallFunction|CreateUIWidgets)
  (CallFunction|BindtoUIEvents)
  (CallFunction|ToggleUIWidgetVisibility (Variables|References|GetMainMenuWidget))
  (CallFunction|SetInputMode)
  (Default|CallUIWidgetsInitialised))

(fn OnCreditsMainMenuClicked
  ;[1 1 1] Close Button Clicked
  (CallFunction|PlaySFXButtonClick (Variables|/Game/Blueprints/BP_GameMode.BP_GameMode_C|GetSFXLowPitch (Variables|References|GetGameMode)))
  (CallFunction|ToggleUIWidgetVisibility (Variables|References|GetCreditsWidget))
  (CallFunction|ToggleUIWidgetVisibility (Variables|References|GetMainMenuWidget)))

(fn OnLearningObjectiveContinueClicked
  ;[1 1 1] Learning Objective Continue Button Clicked
  (CallFunction|StopPlayingNarration)
  (CallFunction|PlaySFXButtonClick 1.0)
  (CallFunction|ToggleUIWidgetVisibility (Variables|References|GetQuestionWidget))
  (CallFunction|ToggleUIWidgetVisibility (Variables|References|GetLearningObjectiveWidget))
  (Default|CallLearningObjectiveContinueClicked))

(fn OnLearningObjectiveLevelSelectClicked
  ;[1 1 1] Level Select Button Clicked
  (CallFunction|StopPlayingNarration)
  (CallFunction|PlaySFXButtonClick (Variables|/Game/Blueprints/BP_GameMode.BP_GameMode_C|GetSFXLowPitch (Variables|References|GetGameMode)))
  (CallFunction|ToggleUIWidgetVisibility (Variables|References|GetLearningObjectiveWidget))
  (CallFunction|ToggleUIWidgetVisibility (Variables|References|GetLevelSelectWidget)))

(fn OnLevelButtonClicked
  (params (LevelIndex :type Integer))
  ;[1 1 1] Level Selected
  (CallFunction|PlaySFXButtonClick 1.0)
  (CallFunction|ToggleUIWidgetVisibility (Variables|References|GetLevelSelectWidget))
  (CallFunction|ToggleUIWidgetVisibility (Variables|References|GetLearningObjectiveWidget))
  (Default|CallLevelSelectionChanged LevelIndex))

(fn OnLevelChanged
  (params (Level :type S%20Level%20Structure))
  ;[1 1 1] On Level Changed
  (CallFunction|PlayLearningMaterialNarration Level))

(fn OnLevelCompleted
  (params (LevelCompleteSummary :type S%20Level%20Complete%20Summary%20Structure))
  ;[1 1 1] Level Completed
  (CallFunction|ToggleUIWidgetVisibility (Variables|References|GetResultWidget))
  (CallFunction|ToggleUIWidgetVisibility (Variables|References|GetLevelCompleteWidget)))

(fn OnLevelCompleteContinueClicked
  ;[1 1 1] Level Complete Continue Button Clicked
  (CallFunction|PlaySFXButtonClick (Variables|/Game/Blueprints/BP_GameMode.BP_GameMode_C|GetSFXLowPitch (Variables|References|GetGameMode)))
  (CallFunction|ToggleUIWidgetVisibility (Variables|References|GetLevelCompleteWidget))
  (CallFunction|ToggleUIWidgetVisibility (Variables|References|GetLearningObjectiveWidget))
  (CallFunction|PlayLearningMaterialNarration)
  (Default|CallLevelSelectionChanged (+ (Variables|/Game/Blueprints/BP_GameMode.BP_GameMode_C|GetCurrentLevelIndex (Variables|References|GetGameMode)) 1)))

(fn OnLevelCompleteLevelSelectClicked
  ;[1 1 1] Level Select Button Clicked
  (CallFunction|PlaySFXButtonClick (Variables|/Game/Blueprints/BP_GameMode.BP_GameMode_C|GetSFXLowPitch (Variables|References|GetGameMode)))
  (CallFunction|ToggleUIWidgetVisibility (Variables|References|GetLevelCompleteWidget))
  (CallFunction|ToggleUIWidgetVisibility (Variables|References|GetLevelSelectWidget)))

(fn OnLevelCompleteMainMenuClicked
  ;[1 1 1] Main Menu Button Clicked
  (CallFunction|PlaySFXButtonClick (Variables|/Game/Blueprints/BP_GameMode.BP_GameMode_C|GetSFXLowPitch (Variables|References|GetGameMode)))
  (CallFunction|ToggleUIWidgetVisibility (Variables|References|GetLevelCompleteWidget))
  (CallFunction|ToggleUIWidgetVisibility (Variables|References|GetMainMenuWidget)))

(fn OnLevelCompleteReplayLevelClicked
  ;[1 1 1] Replay Level Button Clicked
  (CallFunction|PlaySFXButtonClick 1.0)
  (CallFunction|ToggleUIWidgetVisibility (Variables|References|GetLevelCompleteWidget))
  (CallFunction|ToggleUIWidgetVisibility (Variables|References|GetLearningObjectiveWidget))
  (CallFunction|PlayLearningMaterialNarration)
  (Default|CallLevelSelectionChanged (Variables|/Game/Blueprints/BP_GameMode.BP_GameMode_C|GetCurrentLevelIndex (Variables|References|GetGameMode))))

(fn OnLevelSelectMainMenuClicked
  ;[1 1 1] Main Menu Button Clicked
  (CallFunction|PlaySFXButtonClick (Variables|/Game/Blueprints/BP_GameMode.BP_GameMode_C|GetSFXLowPitch (Variables|References|GetGameMode)))
  (CallFunction|ToggleUIWidgetVisibility (Variables|References|GetLevelSelectWidget))
  (CallFunction|ToggleUIWidgetVisibility (Variables|References|GetMainMenuWidget)))

(fn OnMainMenuCreditsClicked
  ;[1 1 1] Credits Button Clicked
  (CallFunction|PlaySFXButtonClick 1.0)
  (CallFunction|ToggleUIWidgetVisibility (Variables|References|GetMainMenuWidget))
  (CallFunction|ToggleUIWidgetVisibility (Variables|References|GetCreditsWidget)))

(fn OnMainMenuOptionsClicked
  ;[1 1 1] Options Button Clicked
  (CallFunction|PlaySFXButtonClick 1.0)
  (CallFunction|ToggleUIWidgetVisibility (Variables|References|GetMainMenuWidget))
  (CallFunction|ToggleUIWidgetVisibility (Variables|References|GetOptionsWidget)))

(fn OnMainMenuPlayClicked
  ;[1 1 1] Play Button Clicked
  (CallFunction|PlaySFXButtonClick 1.0)
  (CallFunction|ToggleUIWidgetVisibility (Variables|References|GetMainMenuWidget))
  (CallFunction|ToggleUIWidgetVisibility (Variables|References|GetLevelSelectWidget)))

(fn OnMainMenuQuitClicked
  ;[1 1 1] Quit Button Clicked
  (CallFunction|PlaySFXButtonClick (Variables|/Game/Blueprints/BP_GameMode.BP_GameMode_C|GetSFXLowPitch (Variables|References|GetGameMode)))
  (Game|QuitGame 0 "Quit" false))

(fn OnNextQuestionSelected
  ;[1 1 1] Next Question Selected
  (CallFunction|ToggleUIWidgetVisibility (Variables|References|GetQuestionWidget))
  (CallFunction|ToggleUIWidgetVisibility (Variables|References|GetResultWidget)))

(fn OnOptionsMainMenuClicked
  ;[1 1 1] Close Button Clicked
  (CallFunction|ToggleUIWidgetVisibility (Variables|References|GetOptionsWidget))
  (CallFunction|ToggleUIWidgetVisibility (Variables|References|GetMainMenuWidget))
  (CallFunction|UpdatePlayerPreferences)
  (CallFunction|ResetProgress))

(fn OnOptionsMusicVolumeChanged
  (params (Volume :type Float%20%28single-precision%29) (IsMuted :type Boolean))
  ;[1 1 1] Raise Event
  (Utilities|Struct|SetmembersinSPlayerPreferences (Variables|Player|GetPlayerPreferences) Volume IsMuted)
  (Default|CallMusicVolumeChanged Volume IsMuted))

(fn OnOptionsNarrationVoiceChanged
  (params (NarrationVoiceType :type ENarrationVoiceTypes%20Enum :default "NewEnumerator0"))
  ;[1 1 1] Update Player Preferences
  (Utilities|Struct|SetmembersinSPlayerPreferences (Variables|Player|GetPlayerPreferences) NarrationVoiceType))

(fn OnOptionsNarrationVolumeChanged
  (params (Volume :type Float%20%28single-precision%29) (IsMuted :type Boolean))
  ;[1 1 1] Raise Event
  (Utilities|Struct|SetmembersinSPlayerPreferences (Variables|Player|GetPlayerPreferences) Volume IsMuted))

(fn OnOptionsSFXVolumeChanged
  (params (Volume :type Float%20%28single-precision%29) (IsMuted :type Boolean))
  ;[1 1 1] Update Player Preferences
  (Utilities|Struct|SetmembersinSPlayerPreferences (Variables|Player|GetPlayerPreferences) Volume IsMuted))

(fn OnPlayerDataLoaded
  (params (PlayerData :type S%20Player%20Data%20Structure) (PlayerPreferences :type S%20Player%20Preferences%20Structure))
  ;[1 1 1] Initialise Player
  (CallFunction|InitialisePlayer PlayerData PlayerPreferences))

(fn OnQuestionAnswerClicked
  (params (IsAnswerCorrect :type Boolean))
  ;[1 1 1] Answer Selected
  (CallFunction|PlaySFXQuestionAnswered IsAnswerCorrect)
  (CallFunction|ToggleUIWidgetVisibility (Variables|References|GetQuestionWidget))
  (CallFunction|ToggleUIWidgetVisibility (Variables|References|GetResultWidget))
  (Default|CallAnswerSelected IsAnswerCorrect))

(fn OnQuestionLevelSelectClicked
  ;[1 1 1] Level Selected Button Clicked
  (CallFunction|ToggleUIWidgetVisibility (Variables|References|GetQuestionWidget))
  (CallFunction|ToggleUIWidgetVisibility (Variables|References|GetLevelSelectWidget)))

(fn OnResultContinueClicked
  ;[1 1 1] Raise Event
  (CallFunction|PlaySFXButtonClick 1.0)
  (Default|CallResultContinueClicked))

(fn OnStarsAwarded
  (params (LevelID :type Integer) (Stars :type Integer))
  ;[1 1 1] Update Level Achievement
  (CallFunction|UpdateLevelAchievement LevelID Stars))

(fn PlayLearningMaterialNarration
  (params (Level :type S%20Level%20Structure))
  (bind _playerpreferences (Variables|Player|GetPlayerPreferences))
  (bind _array_element (Utilities|Array|ForEachLoopwithBreak (.Narration (Utilities|Struct|BreakSLearningMaterial (.LearningMaterial (Utilities|Struct|BreakSLevel Level)))) :!label _label)
    (:LoopBody
      (if (== (.VoiceType (Utilities|Struct|BreakSNarration _array_element)) (.narrationvoicetype _playerpreferences))
        (goto _label Break)))
    (:Completed
      (bind _safevolumemultiplier (Default|GetSafeVolumeMultiplier (Variables|References|GetGameMode) (select (.narrationismuted _playerpreferences) 0.0 (.narrationvolume _playerpreferences))))
      (bind _returnvalue (Audio|SpawnSound2D (.Audio (Utilities|Struct|BreakSNarration _array_element)) _safevolumemultiplier 1.0 0.0 0))
      (Variables|Default|SetNarration _returnvalue))))

(fn PlaySFXButtonClick
  (params (PitchMultiplierOverride :type Float%20%28single-precision%29))
  (bind _playerpreferences (Variables|Player|GetPlayerPreferences))
  ;[1 1 1] Play SFX Button Click
  (bind _safevolumemultiplier (Default|GetSafeVolumeMultiplier (Variables|References|GetGameMode) (select (.sfxismuted _playerpreferences) 0.0 (.sfxvolume _playerpreferences))))
  (Audio|SpawnSound2D (Variables|/Game/Blueprints/BP_GameMode.BP_GameMode_C|GetButtonClickCue (Variables|References|GetGameMode)) _safevolumemultiplier PitchMultiplierOverride 0.0 0))

(fn PlaySFXQuestionAnswered
  (params (IsAnswerCorrect :type Boolean))
  (bind _gamemode (Variables|References|GetGameMode))
  (bind _playerpreferences (Variables|Player|GetPlayerPreferences))
  ;[1 1 1] Play SFX Question Answered (Correctly/Incorrectly)
  (LocalVariables|SetSFXSoundCue (select IsAnswerCorrect (Variables|/Game/Blueprints/BP_GameMode.BP_GameMode_C|GetCorrectAnswerCue _gamemode) (Variables|/Game/Blueprints/BP_GameMode.BP_GameMode_C|GetIncorrectAnswerCue _gamemode)))
  (bind _safevolumemultiplier (Default|GetSafeVolumeMultiplier (Variables|References|GetGameMode) (select (.sfxismuted _playerpreferences) 0.0 (.sfxvolume _playerpreferences))))
  (Audio|SpawnSound2D (LocalVariables|GetSFXSoundCue) _safevolumemultiplier 1.0 0.0 0))

(fn ResetProgress
  ;[1 1 1] Reset Progress
  (if (Default|IsResetProgressChecked (Variables|References|GetOptionsWidget))
    (Default|CallResetPlayerProgressSelected)
    (Default|DeselectResetProgress (Variables|References|GetOptionsWidget))))

(fn SetInputMode
  ;[1 1 1] Set Input Mode
  (Input|SetInputModeUIOnly self (Variables|References|GetMainMenuWidget) "DoNotLock")
  (Variables|/Script/Engine.PlayerController|SetbShowMouseCursor self true))

(fn SetReferences
  ;[1 1 1] Set References
  (bind _asbp_game_mode (Utilities|Casting|CastToBP_GameMode (Game|GetGameMode)))
  (Variables|References|SetGameMode _asbp_game_mode))

(fn StopPlayingNarration
  ;[1 1 1] Stop Playing Narration
  (Utilities|IsValid (Variables|Default|GetNarration)
    (:Is%20Valid
      (if (Audio|Components|Audio|IsPlaying (Variables|Default|GetNarration))
        (Audio|Components|Audio|Stop (Variables|Default|GetNarration))))))

(fn ToggleUIWidgetVisibility
  (params (UserWidget :type User%20Widget%20Object%20Reference))
  ;[1 1 1] Toggle UI Widget Visibility
  (if (Widget|IsVisible UserWidget)
    (Widget|SetVisibility UserWidget "Hidden")
    (else
      (Widget|SetVisibility UserWidget "Visible"))))

(fn UpdateLevelAchievement
  (params (LevelID :type Integer) (Stars :type Integer))
  ;[1 1 1] Update Level Achievement
  (bind _hasachievement (CallFunction|HasLevelAchievementforLevelID LevelID))
  (if _hasachievement
    (bind _index (CallFunction|GetLevelAchievementIndexbyLevelID LevelID))
    (if (< (.Stars (Utilities|Struct|BreakSLevelAchievement (Utilities|Array|Get(acopy) (.levelachievements (Variables|Player|GetPlayerData)) _index))) Stars)
      (Utilities|Struct|SetmembersinSLevelAchievement (Utilities|Array|Get(acopy) (.levelachievements (Variables|Player|GetPlayerData)) _index) Stars)
      (Default|CallLevelAchievementChanged LevelID :!label _label))
    (else
      (Utilities|Array|Add (.levelachievements (Variables|Player|GetPlayerData)) (Utilities|Struct|MakeSLevelAchievement LevelID Stars))
      (goto _label))))

(fn UpdatePlayerPreferences
  ;[1 1 1] Update Player Preferences
  (bind _playerpreferences (Default|GetPlayerPreferences (Variables|References|GetOptionsWidget)))
  (Variables|Player|SetPlayerPreferences _playerpreferences)
  (Default|CallPlayerPreferencesChanged))