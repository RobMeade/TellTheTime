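; Player controller for a level-based quiz game that owns the UI flow and the player's stars and highest unlocked level.
; InitialiseUI creates all screen widgets and the HUD, binds their events and sets UI-only input.
; Menu clicks and GameMode events toggle screen visibility from menus through objective, question, result and level completion.
; It initialises progress from loaded player data and relays selections and progress changes through event dispatchers.
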(event EventBeginPlay
  ;[1 1 1] Initialise
  (CallFunction|SetReferences)
  (CallFunction|BindtoGameModeEvents)
  (Default|CallPlayerControllerInitialised))

(fn ConstructionScript)

(fn SetReferences
  ;[1 1 1] Set References
  (bind _asbp_game_mode (Utilities|Casting|CastToBP_GameMode (Game|GetGameMode)))
  (Variables|References|SetGameMode _asbp_game_mode))

(fn BindtoGameModeEvents
  ;[1 1 1] Bind to GameMode Events
  (EventDispatchers|BindEventtoLevelDataLoaded (Variables|References|GetGameMode) (EventDispatchers|CreateEvent :!event OnLevelDataLoaded))
  (EventDispatchers|BindEventtoPlayerDataLoaded (Variables|References|GetGameMode) (EventDispatchers|CreateEvent :!event OnPlayerDataLoaded))
  (EventDispatchers|BindEventtoNextQuestionSelected (Variables|References|GetGameMode) (EventDispatchers|CreateEvent :!event OnNextQuestionSelected))
  (EventDispatchers|BindEventtoLevelCompleted (Variables|References|GetGameMode) (EventDispatchers|CreateEvent :!event OnLevelCompleted)))

(fn InitialiseUI
  ;[1 1 1] Initialise UI
  (CallFunction|CreateUIWidgets)
  (CallFunction|BindtoUIEvents)
  (CallFunction|ToggleUIWidgetVisibility (Variables|References|GetMainMenuWidget))
  (CallFunction|SetInputMode)
  (Default|CallUIWidgetsInitialised))

(fn CreateUIWidgets
  ;[1 1 1] Create UI Widgets
  (bind _returnvalue (UserInterface|CreateWidget "/Game/WBP_MainMenu.WBP_MainMenu_C" self))
  (bind _output_get (Variables|References|SetMainMenuWidget _returnvalue))
  (CallFunction|AddtoViewportandHide _output_get)
  (bind _returnvalue_2 (UserInterface|CreateWidget "/Game/WBP_Options.WBP_Options_C" self))
  (bind _output_get_2 (Variables|References|SetOptionsWidget _returnvalue_2))
  (CallFunction|AddtoViewportandHide _output_get_2)
  (bind _returnvalue_3 (UserInterface|CreateWidget "/Game/WBP_LevelSelect.WBP_LevelSelect_C" self))
  (bind _output_get_3 (Variables|References|SetLevelSelectWidget _returnvalue_3))
  (CallFunction|AddtoViewportandHide _output_get_3)
  (bind _returnvalue_4 (UserInterface|CreateWidget "/Game/WBP_LearningObjective.WBP_LearningObjective_C" self))
  (bind _output_get_4 (Variables|References|SetLearningObjectiveWidget _returnvalue_4))
  (CallFunction|AddtoViewportandHide _output_get_4)
  (bind _returnvalue_5 (UserInterface|CreateWidget "/Game/WBP_Question.WBP_Question_C" self))
  (bind _output_get_5 (Variables|References|SetQuestionWidget _returnvalue_5))
  (CallFunction|AddtoViewportandHide _output_get_5)
  (bind _returnvalue_6 (UserInterface|CreateWidget "/Game/WBP_Result.WBP_Result_C" self))
  (bind _output_get_6 (Variables|References|SetResultWidget _returnvalue_6))
  (CallFunction|AddtoViewportandHide _output_get_6)
  (bind _returnvalue_7 (UserInterface|CreateWidget "/Game/WBP_LevelComplete.WBP_LevelComplete_C" self))
  (bind _output_get_7 (Variables|References|SetLevelCompleteWidget _returnvalue_7))
  (CallFunction|AddtoViewportandHide _output_get_7)
  (bind _returnvalue_8 (UserInterface|CreateWidget "/Game/WBP_HUD.WBP_HUD_C" self))
  (bind _output_get_8 (Variables|References|SetHUDWidget _returnvalue_8))
  (UserInterface|Viewport|AddtoViewport _output_get_8 0))

(fn AddtoViewportandHide
  (params (UserWidget :type User%20Widget%20Object%20Reference))
  ;[1 1 1] Add to Viewport and Hide
  (UserInterface|Viewport|AddtoViewport UserWidget 0)
  (Widget|SetVisibility UserWidget "Hidden"))

(fn BindtoUIEvents
  ;[1 1 1] Bind to UI Events
  (EventDispatchers|BindEventtoPlayClicked (Variables|References|GetMainMenuWidget) (EventDispatchers|CreateEvent :!event OnMainMenuPlayClicked))
  (EventDispatchers|BindEventtoOptionsClicked (Variables|References|GetMainMenuWidget) (EventDispatchers|CreateEvent :!event OnMainMenuOptionsClicked))
  (EventDispatchers|BindEventtoQuitClicked (Variables|References|GetMainMenuWidget) (EventDispatchers|CreateEvent :!event OnMainMenuQuitClicked))
  (EventDispatchers|BindEventtoCloseClicked (Variables|References|GetOptionsWidget) (EventDispatchers|CreateEvent :!event OnOptionsCloseClicked))
  (EventDispatchers|BindEventtoMainMenuClicked (Variables|References|GetLevelSelectWidget) (EventDispatchers|CreateEvent :!event OnLevelSelectMainMenuClicked))
  (EventDispatchers|BindEventtoLevelSelected (Variables|References|GetLevelSelectWidget) (EventDispatchers|CreateEvent :!event OnLevelButtonClicked))
  (EventDispatchers|BindEventtoContinueClicked (Variables|References|GetLearningObjectiveWidget) (EventDispatchers|CreateEvent :!event OnLearningObjectiveContinueClicked))
  (EventDispatchers|BindEventtoAnswerSelected (Variables|References|GetQuestionWidget) (EventDispatchers|CreateEvent :!event OnQuestionAnswerClicked))
  (EventDispatchers|BindEventtoOnContinueClicked (Variables|References|GetResultWidget) (EventDispatchers|CreateEvent :!event OnResultContinueClicked))
  (EventDispatchers|BindEventtoOnContinueClicked (Variables|References|GetLevelCompleteWidget) (EventDispatchers|CreateEvent :!event OnLevelCompleteContinueClicked)))

(fn ToggleUIWidgetVisibility
  (params (UserWidget :type User%20Widget%20Object%20Reference))
  ;[1 1 1] Toggle UI Widget Visibility
  (if (Widget|IsVisible UserWidget)
    (Widget|SetVisibility UserWidget "Hidden")
    (else
      (Widget|SetVisibility UserWidget "Visible"))))

(fn SetInputMode
  ;[1 1 1] Set Input Mode
  (Input|SetInputModeUIOnly self (Variables|References|GetMainMenuWidget) "DoNotLock")
  (Variables|/Script/Engine.PlayerController|SetbShowMouseCursor self true))

(fn OnLevelDataLoaded
  ;[1 1 1] Raise Event
  (Default|CallLevelDataLoaded))

(fn OnPlayerDataLoaded
  (params (PlayerData :type S%20Player%20Data%20Structure))
  ;[1 1 1] Initialise Player
  (CallFunction|InitialisePlayer PlayerData))

(fn OnMainMenuPlayClicked
  ;[1 1 1] Play Button Clicked
  (CallFunction|ToggleUIWidgetVisibility (Variables|References|GetMainMenuWidget))
  (CallFunction|ToggleUIWidgetVisibility (Variables|References|GetLevelSelectWidget)))

(fn OnMainMenuOptionsClicked
  ;[1 1 1] Option Button Clicked
  (CallFunction|ToggleUIWidgetVisibility (Variables|References|GetMainMenuWidget))
  (CallFunction|ToggleUIWidgetVisibility (Variables|References|GetOptionsWidget)))

(fn OnMainMenuQuitClicked
  ;[1 1 1] Quit Button Clicked
  (Game|QuitGame 0 "Quit" false))

(fn OnOptionsCloseClicked
  ;[1 1 1] Close Button Clicked
  (CallFunction|ToggleUIWidgetVisibility (Variables|References|GetOptionsWidget))
  (CallFunction|ToggleUIWidgetVisibility (Variables|References|GetMainMenuWidget)))

(fn InitialisePlayer
  (params (PlayerData :type S%20Player%20Data%20Structure))
  (bind (_stars _highestlevelunlocked) (Utilities|Struct|BreakSPlayerData PlayerData))
  ;[1 1 1] Initialise Player
  (bind _output_get (Variables|Default|SetStars _stars))
  (Default|CallPlayerStarsChanged _output_get)
  (bind _output_get_2 (Variables|Default|SetHighestLevelUnlocked _highestlevelunlocked))
  (Default|CallPlayerHighestLevelUnlockedChanged _output_get_2))

(fn OnLevelSelectMainMenuClicked
  ;[1 1 1] Main Menu Button Clicked
  (CallFunction|ToggleUIWidgetVisibility (Variables|References|GetLevelSelectWidget))
  (CallFunction|ToggleUIWidgetVisibility (Variables|References|GetMainMenuWidget)))

(fn IncrementStars
  ;[1 1 1] Increment Player Stars
  (bind _result (Math|Integer|IncrementInt (Variables|Default|GetStars))
    (:%20%20
      (Default|CallPlayerStarsChanged _result))))

(fn OnLevelButtonClicked
  (params (LevelIndex :type Integer))
  ;[1 1 1] Level Selected
  (CallFunction|ToggleUIWidgetVisibility (Variables|References|GetLevelSelectWidget))
  (CallFunction|ToggleUIWidgetVisibility (Variables|References|GetLearningObjectiveWidget))
  (Default|CallLevelSelectionChanged LevelIndex))

(fn OnLearningObjectiveContinueClicked
  ;[1 1 1] Learning Objective Continue Button Clicked
  (CallFunction|ToggleUIWidgetVisibility (Variables|References|GetQuestionWidget))
  (CallFunction|ToggleUIWidgetVisibility (Variables|References|GetLearningObjectiveWidget))
  (Default|CallLearningObjectiveContinueClicked))

(fn OnQuestionAnswerClicked
  (params (IsAnswerCorrect :type Boolean))
  ;[1 1 1] Answer Selected
  (CallFunction|ToggleUIWidgetVisibility (Variables|References|GetQuestionWidget))
  (CallFunction|ToggleUIWidgetVisibility (Variables|References|GetResultWidget))
  (Default|CallAnswerSelected IsAnswerCorrect))

(fn OnResultContinueClicked
  ;[1 1 1] Raise Event
  (Default|CallResultContinueClicked))

(fn OnNextQuestionSelected
  ;[1 1 1] Next Question Selected
  (CallFunction|ToggleUIWidgetVisibility (Variables|References|GetQuestionWidget))
  (CallFunction|ToggleUIWidgetVisibility (Variables|References|GetResultWidget)))

(fn OnLevelCompleted
  (params (UnlockedLevelID :type Integer) (AreMoreLevels :type Boolean))
  ;[1 1 1] Level Completed
  (CallFunction|ToggleUIWidgetVisibility (Variables|References|GetResultWidget))
  (CallFunction|ToggleUIWidgetVisibility (Variables|References|GetLevelCompleteWidget)))

(fn OnLevelCompleteContinueClicked
  (CallFunction|ToggleUIWidgetVisibility (Variables|References|GetLevelCompleteWidget))
  (CallFunction|ToggleUIWidgetVisibility (Variables|References|GetLevelSelectWidget)))

(fn IncrementHighestLevelUnlocked
  ;[1 1 1] Increment Highest Level Unlocked
  (bind _result (Math|Integer|IncrementInt (Variables|Default|GetHighestLevelUnlocked))
    (:%20%20
      (Default|CallPlayerHighestLevelUnlockedChanged _result))))