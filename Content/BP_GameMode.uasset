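; Game mode for a level-based quiz game, running question progression, star awards, level unlocks and saving.
; It binds to player controller events, starting a chain that initialises UI, loads save data and reads levels from a data table.
; Level, answer and continue events advance the game state, which it broadcasts through dispatcher calls.
; Progress saves on level completion, preference changes or reset; volume handlers only print debug text.
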(event EventBeginPlay
  ;[1 1 1] Initialise
  (CallFunction|SetReferences)
  (CallFunction|BindtoEvents))

(fn ConstructionScript)

(fn SetReferences
  ;[1 1 1] Set References
  (bind _asbp_player_controller (Utilities|Casting|CastToBP_PlayerController (Game|GetPlayerController 0)))
  (Variables|Default|SetPlayerController _asbp_player_controller)
  (bind _returnvalue (SaveGame|CreateSaveGameObject "/Game/SG_SaveGame.SG_SaveGame_C"))
  (Variables|Default|SetSaveGame _returnvalue))

(fn BindtoEvents
  ;[1 1 1] Bind to Events
  (EventDispatchers|BindEventtoPlayerControllerInitialised (Variables|Default|GetPlayerController) (EventDispatchers|CreateEvent :!event OnPlayerControllerInitialised))
  (EventDispatchers|BindEventtoUIWidgetsInitialised (Variables|Default|GetPlayerController) (EventDispatchers|CreateEvent :!event OnUIWidgetsInitialised))
  (EventDispatchers|BindEventtoLevelSelectionChanged (Variables|Default|GetPlayerController) (EventDispatchers|CreateEvent :!event OnLevelSelectionChanged))
  (EventDispatchers|BindEventtoLearningObjectiveContinueClicked (Variables|Default|GetPlayerController) (EventDispatchers|CreateEvent :!event OnLearningObjectiveContinueClicked))
  (EventDispatchers|BindEventtoAnswerSelected (Variables|Default|GetPlayerController) (EventDispatchers|CreateEvent :!event OnAnswerSelected))
  (EventDispatchers|BindEventtoResultContinueClicked (Variables|Default|GetPlayerController) (EventDispatchers|CreateEvent :!event OnResultContinueClicked))
  (EventDispatchers|BindEventtoMusicVolumeChanged (Variables|Default|GetPlayerController) (EventDispatchers|CreateEvent :!event OnMusicVolumeChanged))
  (EventDispatchers|BindEventtoSFXVolumeChanged (Variables|Default|GetPlayerController) (EventDispatchers|CreateEvent :!event OnSFXVolumeChanged))
  (EventDispatchers|BindEventtoNarrationVolumeChanged (Variables|Default|GetPlayerController) (EventDispatchers|CreateEvent :!event OnNarrationVolumeChanged))
  (EventDispatchers|BindEventtoPlayerPreferencesChanged (Variables|Default|GetPlayerController) (EventDispatchers|CreateEvent :!event OnPlayerPreferencesChanged))
  (EventDispatchers|BindEventtoResetPlayerProgressSelected (Variables|Default|GetPlayerController) (EventDispatchers|CreateEvent :!event OnResetPlayerProgress)))

(fn LoadLevelData
  ;[1 1 1] Load Level Data
  (bind _outrownames (DataTable|GetDataTableRowNames "/Game/DT_Levels.DT_Levels"))
  (for _array_element _outrownames
    (bind _returnvalue (Utilities|GetDataTableRow "/Game/DT_Levels.DT_Levels" _array_element)
      (:then
        (Utilities|Array|Add (Variables|Default|GetLevels) _returnvalue))))
  (Default|CallLevelDataLoaded))

(fn LoadPlayerData
  (bind _savegame (Variables|Default|GetSaveGame))
  ;[1 1 1] Load Player Data
  (Default|LoadData (Variables|Default|GetSaveGame))
  (Default|CallPlayerDataLoaded (Variables|/Game/SG_SaveGame.SG_SaveGame_C|GetPlayerData _savegame) (Variables|/Game/SG_SaveGame.SG_SaveGame_C|GetPlayerPreferences _savegame)))

(fn InitialiseUI
  ;[1 1 1] Initialise UI
  (Default|InitialiseUI (Variables|Default|GetPlayerController)))

(fn OnPlayerControllerInitialised
  ;[1 1 1] Initialise UI
  (CallFunction|InitialiseUI))

(fn OnUIWidgetsInitialised
  ;[1 1 1] Initialise Game
  (CallFunction|InitialiseGame))

(fn InitialiseGame
  ;[1 1 1] Initialise Game
  (CallFunction|InitialiseSaveGame)
  (CallFunction|LoadPlayerData)
  (CallFunction|LoadLevelData))

(fn OnLevelSelectionChanged
  (params (LevelIndex :type Integer))
  ;[1 1 1] Level Selection Changed
  (bind _output_get (Variables|Default|SetCurrentLevelIndex LevelIndex))
  (bind _level (CallFunction|GetLevelbyIndex _output_get))
  (bind _output_get_2 (Variables|Default|SetCurrentLevel _level))
  (Variables|Default|SetCurrentQuestionIndex 0)
  (Default|CallLevelChanged _output_get_2))

(fn OnLearningObjectiveContinueClicked
  ;[1 1 1] Learning Objective Continue Clicked
  (bind _question (CallFunction|GetQuestion))
  (Default|CallQuestionChanged _question))

(fn GetLevelbyIndex
  (params (Index :type Integer))
  ;[1 1 1] Get Level by Index
  (return (Utilities|Array|Get(acopy) (Variables|Default|GetLevels) Index)))

(fn GetQuestion
  ;[1 1 1] Get Question
  (return (Utilities|Array|Get(acopy) (.Questions (Utilities|Struct|BreakSLevel (Variables|Default|GetCurrentLevel))) (Variables|Default|GetCurrentQuestionIndex))))

(fn OnAnswerSelected
  (params (IsAnswerCorrect :type Boolean))
  ;[1 1 1] Answer Selected
  (if IsAnswerCorrect
    (Default|IncrementStars (Variables|Default|GetPlayerController)))
  (Default|CallResultChanged IsAnswerCorrect))

(fn OnResultContinueClicked
  (bind _playercontroller (Variables|Default|GetPlayerController))
  (bind _morequestions (CallFunction|LevelHasMoreQuestions))
  (if _morequestions
    (Math|Integer|IncrementInt (Variables|Default|GetCurrentQuestionIndex)
      (:%20%20
        (bind _question (CallFunction|GetQuestion))
        (Default|CallQuestionChanged _question)
        (Default|CallNextQuestionSelected)))
    (else
      (bind _morelevel (CallFunction|GameHasMoreLevels))
      (Default|IncrementHighestLevelUnlocked _playercontroller)
      (CallFunction|SavePlayerData)
      (Default|CallLevelCompleted (.highestlevelunlocked (Variables|/Game/BP_PlayerController.BP_PlayerController_C|GetPlayerData _playercontroller)) _morelevel))))

(fn LevelHasMoreQuestions
  ;[1 1 1] Level Has More Questions?
  (return (< (Variables|Default|GetCurrentQuestionIndex) (Utilities|Array|LastIndex (.Questions (Utilities|Struct|BreakSLevel (Variables|Default|GetCurrentLevel)))))))

(fn GameHasMoreLevels
  ;[1 1 1] Game Has More Levels?
  (return (< (Variables|Default|GetCurrentLevelIndex) (Utilities|Array|LastIndex (Variables|Default|GetLevels)))))

(fn GetDefaultPlayerData
  ;[1 1 1] Get Default Player Data
  (return (Utilities|Struct|MakeSPlayerData (Variables|Config|Game|GetDefaultPlayerStars) (Variables|Config|Game|GetDefaultLevelUnlocked)) (Utilities|Struct|MakeSPlayerPreferences (Variables|Config|Audio|GetDefaultMusicVolume) false (Variables|Config|Audio|GetDefaultSFXVolume) false (Variables|Config|Audio|GetDefaultNarrationVolume))))

(fn OnMusicVolumeChanged
  (params (Volume :type Float%20%28single-precision%29))
  (Development|PrintString (Utilities|String|Append "Music Volume : " (Utilities|String|ToString(Float) Volume)) true true "(R=0.000000,G=0.660000,B=1.000000,A=1.000000)" 0.5))

(fn OnSFXVolumeChanged
  (params (Volume :type Float%20%28single-precision%29))
  (Development|PrintString (Utilities|String|Append "SFX Volume : " (Utilities|String|ToString(Float) Volume)) true true "(R=0.000000,G=0.660000,B=1.000000,A=1.000000)" 0.5))

(fn OnNarrationVolumeChanged
  (params (Volume :type Float%20%28single-precision%29))
  (Development|PrintString (Utilities|String|Append "Narration : " (Utilities|String|ToString(Float) Volume)) true true "(R=0.000000,G=0.660000,B=1.000000,A=1.000000)" 0.5))

(fn OnPlayerPreferencesChanged
  ;[1 1 1] Save Player Data
  (CallFunction|SavePlayerData))

(fn SavePlayerData
  (bind _playercontroller (Variables|Default|GetPlayerController))
  ;[1 1 1] Save Player Data
  (Default|SaveData (Variables|Default|GetSaveGame) (Variables|/Game/BP_PlayerController.BP_PlayerController_C|GetPlayerData _playercontroller) (Variables|/Game/BP_PlayerController.BP_PlayerController_C|GetPlayerPreferences _playercontroller)))

(fn InitialiseSaveGame
  ;[1 1 1] Initialise Save Game
  (bind (_playerdata _playerpreferences) (CallFunction|GetDefaultPlayerData))
  (Default|Initialise (Variables|Default|GetSaveGame) _playerdata _playerpreferences))

(fn OnResetPlayerProgress
  (bind _playercontroller (Variables|Default|GetPlayerController))
  (bind _playercontroller_2 (Variables|Default|GetPlayerController))
  (bind _playerdata (CallFunction|GetDefaultPlayerData))
  (bind _output_get (Variables|/Game/BP_PlayerController.BP_PlayerController_C|SetPlayerData _playercontroller _playerdata))
  (Default|SaveData (Variables|Default|GetSaveGame) _output_get (Variables|/Game/BP_PlayerController.BP_PlayerController_C|GetPlayerPreferences _playercontroller))
  (Default|CallPlayerDataLoaded (Variables|/Game/BP_PlayerController.BP_PlayerController_C|GetPlayerData _playercontroller_2) (Variables|/Game/BP_PlayerController.BP_PlayerController_C|GetPlayerPreferences _playercontroller_2)))